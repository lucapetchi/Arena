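; BP_AI is a pistol-armed enemy pawn that wanders, chases the player and shoots.
; It loops random reachable-point moves until PawnSensing spots a BP_FirstPersonCharacter, then moves within range of it.
; On arrival it faces the target and fires one damaging line trace from the muzzle along the mesh's right vector, with flash and sound.
; Incoming damage lowers Health, and depletion only turns on mesh physics, without stopping the AI logic.
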(event `self.ReceiveBeginPlay`
  (`self.Search Around`))

(event `Search Around`
  ; Search Around
  (`|AIMoveTo` self (`NavigationSystemV1.K2_GetRandomReachablePointInRadius` (`self.K2_GetActorLocation`) 2000.0 null null) null 300.0
    (:`OnSuccess`
      (`KismetSystemLibrary.Delay` 1.2)
      (`self.Search Around`))))

(event `self.ReceiveAnyDamage`
  (params (Damage :type "Float (single-precision)") (DamageType :type "DamageType Object Reference") (InstigatedBy :type "Controller Object Reference") (DamageCauser :type "Actor Object Reference"))
  ; Health
  (set `self.Health` (- (`self.Health`) Damage))
  (if (<= (`self.Health`) 0.0)
    (`PrimitiveComponent.SetSimulatePhysics` (`self.Mesh`) true)))

(event `self.PawnSensing.OnSeePawn`
  (params (Pawn :type "Pawn Object Reference"))
  (cast `/Game/FirstPerson/Blueprints/BP_FirstPersonCharacter` Pawn)
  (`self.Chase Target` Pawn))

(event `Chase Target`
  (params (TargetActor :type "Actor Object Reference"))
  (`|AIMoveTo` self (0.0 0.0 0.0) TargetActor 1000.0
    (:`OnSuccess`
      (`self.Fire` TargetActor))))

(event `Fire`
  (params (Target :type "Actor Object Reference"))
  (bind _returnvalue_location (`KismetMathLibrary.BreakTransform` (`SceneComponent.GetSocketTransform` (`self.Pistol`) "Muzzle" "RTS_World")))
  (`Controller.SetControlRotation` (`self.GetController`) (`KismetMathLibrary.FindLookAtRotation` (`self.K2_GetActorLocation`) (`self.K2_GetActorLocation` Target)))
  (`|ExecutionSequence`
    (:`then_0`
      (bind (_outhit _returnvalue) (`KismetSystemLibrary.LineTraceSingle` :`Start` _returnvalue_location :`End` (+ _returnvalue_location (* (`KismetMathLibrary.GetRightVector` (`SceneComponent.K2_GetComponentRotation` (`self.Mesh`))) 5000.0)) :`TraceChannel` "TraceTypeQuery1" :`DrawDebugType` "ForDuration"))
      (if _returnvalue
        (`GameplayStatics.ApplyDamage` (`.HitActor` (`GameplayStatics.BreakHitResult` _outhit)) 15.0)))
    (:`then_1`
      (`GameplayStatics.SpawnEmitterAttached` "/Game/StarterContent/Particles/P_MuzzleFlash.P_MuzzleFlash" (`self.Pistol`) "Muzzle" (0.0 0.0 0.0) (struct) (0.1 0.1 0.1) "KeepRelativeOffset" true "AutoRelease")
      (`GameplayStatics.PlaySoundAtLocation` "/Game/Audio/MS_PistolFire.MS_PistolFire" (`self.K2_GetActorLocation`) (struct) 1.0 1.0 0.0 null null null null))))

(fn `UserConstructionScript`)