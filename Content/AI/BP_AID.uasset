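; BP_AID is an AI character that takes damage, dies into a ragdoll and performs a melee attack.
; Damage reduces Health; at zero or below it enables mesh physics, disables movement and increments Kills on the player's BP_FirstPersonCharacter, with no guard against repeat counting.
; While alive, Attack plays a montage whose notify triggers a short forward sphere trace against Pawns, applying fixed damage to the hit actor.
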(event `self.ReceiveAnyDamage`
  (params (Damage :type "Float (single-precision)") (DamageType :type "DamageType Object Reference") (InstigatedBy :type "Controller Object Reference") (DamageCauser :type "Actor Object Reference"))
  (set `self.Health` (- (`self.Health`) Damage))
  (if (<= (`self.Health`) 0.0)
    (`PrimitiveComponent.SetSimulatePhysics` (`self.Mesh`) true)
    (`|ExecutionSequence`
      (:`then_0`
        (set `self.IsDead` true)
        (`CharacterMovementComponent.DisableMovement` (`self.CharacterMovement`)))
      (:`then_1`
        (bind _asbp_first_person_character (cast `/Game/FirstPerson/Blueprints/BP_FirstPersonCharacter` (`GameplayStatics.GetPlayerCharacter` 0)))
        (`/Engine/EditorBlueprintResources/StandardMacros.IncrementInt` (`/Game/FirstPerson/Blueprints/BP_FirstPersonCharacter.Kills` _asbp_first_person_character))))))

(event `/Game/AI/BPI_AI.Attack`
  (bind _returnvalue (`self.K2_GetActorLocation`))
  (if (not (`self.IsDead`))
    (`|PlayMontage` (`self.Mesh`) "/Game/Characters/Mannequins/Animations/Attack_Montage.Attack_Montage"
      (:`OnNotifyBegin`
        (bind (_outhit _returnvalue_2) (`KismetSystemLibrary.SphereTraceSingleForObjects` _returnvalue (+ (* (`KismetMathLibrary.GetForwardVector` (`self.K2_GetActorRotation`)) 170.0) _returnvalue) 30.0 (`|MakeArray` "ObjectTypeQuery3" :!type "EObjectTypeQuery Enum")))
        (if _returnvalue_2
          (`GameplayStatics.ApplyDamage` (`.HitActor` (`GameplayStatics.BreakHitResult` _outhit)) 10.0))))))

(fn `UserConstructionScript`)